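; PlatformBP is a jump platform that spawns another copy of itself when a ThrowOrb_BP overlaps its Trigger.
; A debug input action A runs the same spawn.
; GetLoc picks the new location from random distance and height ranges added to the actor's position.
; A random sign multiplies the whole world X and Y values, so results can mirror across the world origin rather than around the platform.
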(event OnComponentBeginOverlap(trigger)
  (params (OverlappedComponent :type Primitive%20Component%20Object%20Reference) (OtherActor :type Actor%20Object%20Reference) (OtherComp :type Primitive%20Component%20Object%20Reference) (OtherBodyIndex :type Integer) (bFromSweep :type Boolean) (SweepResult :type Hit%20Result%20Structure%20%28by%20ref%29))
  (Utilities|Casting|CastToThrowOrb_BP OtherActor)
  (bind _loc (CallFunction|GetLoc))
  (Game|SpawnActorfromClass "PlatformBP_C" (Math|Transform|MakeTransform _loc "0, 0, 0" "3.000000,3.000000,0.750000") "Undefined" 0 0))

(event EventBeginPlay)

(event Collision|EventActorBeginOverlap
  (params (OtherActor :type Actor%20Object%20Reference)))

(event EventTick
  (params (DeltaSeconds :type Float%20%28single-precision%29)))

(event Input|ActionEvents|InputActionA
  (params (Key :type Key%20Structure :default "None"))
  (:Pressed
    (bind _loc (CallFunction|GetLoc))
    (Game|SpawnActorfromClass "PlatformBP_C" (Math|Transform|MakeTransform _loc "0, 0, 0" "3.000000,3.000000,0.750000") "Undefined" 0 0)))

(fn ConstructionScript)

(fn GetLoc
  (bind _returnvalue (Transformation|GetActorLocation))
  (bind _closedist (Variables|Default|GetcloseDist))
  (bind _fardist (Variables|Default|GetfarDist))
  (return (Math|Vector|MakeVector (* (Math|Random|RandomFloatinRange (+ (.x _returnvalue) _closedist) (+ (.x _returnvalue) _fardist)) (Math|Float|Sign(Float) (Math|Random|RandomFloatinRange -1.0 1.0))) (* (Math|Random|RandomFloatinRange (+ (.y _returnvalue) _closedist) (+ (.y _returnvalue) _fardist)) (Math|Float|Sign(Float) (Math|Random|RandomFloatinRange -1.0 1.0))) (Math|Random|RandomFloatinRange (+ (.z _returnvalue) (Variables|Default|GetcloseHeight)) (+ (.z _returnvalue) (Variables|Default|GetfarHeight))))))